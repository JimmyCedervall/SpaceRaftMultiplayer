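; BP_ItemSpawner is an actor that continuously spawns random pickups inside a box volume.
; A looping one-second timer started on BeginPlay calls Server_SpawnItem, which picks a random row from the DT_Spawnables data table.
; The row's PickupClass spawns at a random point within the configured box, adjusting for collisions but always spawning.
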(event Custom|Server_SpawnItem
  (bind _outrownames (DataTable|GetDataTableRowNames "/Game/Inventory/DT_Spawnables.DT_Spawnables"))
  (bind _output_get (Variables|Default|SetAllSpawnables _outrownames)) ; Kanske kan byta namn på DT till spacedebris eller något
  (bind _returnvalue (Utilities|GetDataTableRow "/Game/Inventory/DT_Spawnables.DT_Spawnables" (Utilities|Array|Get(acopy) _output_get (- (Math|Random|RandomIntegerinRange 1 (Utilities|Array|Length (Variables|Default|GetAllSpawnables))) 1)))
    (:then
      (Game|SpawnActorfromClass (.PickupClass (Utilities|Struct|BreakST_Item _returnvalue)) (Math|Conversions|ToTransform(Vector) (Math|Random|RandomPointinBoundingBox (Variables|Default|GetSpawnBoxPosition) (Variables|Default|GetSpawnBoxExtent))) "AdjustIfPossibleButAlwaysSpawn" 0 0))))

(event EventBeginPlay
  (Utilities|Time|SetTimerbyEvent (delegate Custom|Server_SpawnItem) 1.0 true))

(fn ConstructionScript)