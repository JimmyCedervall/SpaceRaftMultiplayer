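; Base actor for networked pickups, including weapons, that exposes item type, ID, weapon type, blendspace, ammo and pickup state through getters.
; Fire, start-fire and stop-fire events forward to server events left empty as override points, and ammo info returns zero.
; On the authority, sphere overlap by a Player-tagged actor passes the pickup to it after a short workaround delay.
; Server events disable collision and pickup availability, or destroy the actor.
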(event OnComponentBeginOverlap(Sphere)
  (params (OverlappedComponent :type Primitive%20Component%20Object%20Reference) (OtherActor :type Actor%20Object%20Reference) (OtherComp :type Primitive%20Component%20Object%20Reference) (OtherBodyIndex :type Integer) (bFromSweep :type Boolean) (SweepResult :type Hit%20Result%20Structure%20%28by%20ref%29))
  (Networking|SwitchHasAuthority
    (:Authority
      (if (Actor|ActorHasTag OtherActor "Player")
        (Utilities|FlowControl|Delay 0.2) ; Fixes Weird bug
        (Class|INTSurvivalCharacter|SetPickup(Message) OtherActor self)))))

(event OnComponentEndOverlap(Sphere)
  (params (OverlappedComponent :type Primitive%20Component%20Object%20Reference) (OtherActor :type Actor%20Object%20Reference) (OtherComp :type Primitive%20Component%20Object%20Reference) (OtherBodyIndex :type Integer))
  (Networking|SwitchHasAuthority))

(event Custom|Server_RemovePickupFromWorld
  (Actor|DestroyActor))

(event Custom|Server_DisableCollision
  (Collision|SetCollisionEnabled (Variables|Default|GetSphere) "NoCollision")
  (Variables|Default|SetCanBePickedUp false))

(event Custom|Server_FireWeapon
  ;[1 1 1] Fire The Weapon Override
)

(event Custom|Server_StartFire
  ;[1 1 1] Fire The Weapon Override
)

(event Custom|Server_StopFire
  ;[1 1 1] Fire The Weapon Override
)

(event EventStartFire
  ;[1 1 1] Fire The Weapon Override
  (CallFunction|ServerStartFire))

(event EventStopFire
  ;[1 1 1] Fire The Weapon Override
  (CallFunction|ServerStopFire))

(event EventFireWeapon
  ;[1 1 1] Fire The Weapon Override
  (CallFunction|ServerFireWeapon))

(fn ConstructionScript)

(fn BlendspaceInt
  (return (Variables|Default|GetBlendspace)))

(fn GetAmmoInfo
  (return 0 0))

(fn GetItemType
  (return (Variables|Default|GetItemType)))

(fn GetPickupInfo
  (return (Variables|Default|GetItemID)))

(fn GetPickupState
  (return (Variables|Default|GetCanBePickedUp)))

(fn GetWeaponType
  (return (Variables|Default|GetWeaponType)))

(fn PickupRef
  (return self))