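; Player controller for a survival game, linking the player to the HUD and inventory.
; It creates PlayerUI on the local client and forwards health, thirst, hunger, stamina, pickup text and ammo updates, with ammo routed through client events.
; The Inventory input toggles the ACInventory widget, cursor and input mode.
; Pickups resolve to DT_Items rows, are added through a server event and destroyed when fully added; drop events remove or spawn items.
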(event Custom|Server_AddInventoryItem
  (params (Item%20to%20Add :type ST%20Item%20Structure%20%28by%20ref%29) (Pickup :type Actor%20Object%20Reference))
  (bind _all_added (Default|InventoryAddItem(Server) (Variables|Default|GetAC_Inventory) Item%20to%20Add))
  (if _all_added
    (Actor|DestroyActor Pickup)))

(event Custom|Client_SetMaxAmmoUI
  (params (MaxAmmo :type Integer))
  (Default|SetMaxAmmo (Variables|Default|GetPlayerUI) MaxAmmo))

(event Custom|Client_UpdateAmmoUI
  (params (CurrentAmmo :type Integer))
  (Default|UpdateAmmo (Variables|Default|GetPlayerUI) CurrentAmmo))

(event EventUpdateHealthUI
  (params (NewHealth :type Float%20%28single-precision%29))
  (Default|UpdateHealth (Variables|Default|GetPlayerUI) NewHealth))

(event EventUpdateStaminaUI
  (params (NewStamina :type Float%20%28single-precision%29))
  (Default|UpdateStamina (Variables|Default|GetPlayerUI) NewStamina))

(event EventUpdatePickupText
  (params (PickupText :type Text) (Visibility :type ESlateVisibility%20Enum :default "Visible"))
  (Default|UpdatePickupText (Variables|Default|GetPlayerUI) PickupText Visibility))

(event EventBeginPlay
  (if (Pawn|IsLocalPlayerController) ; Make sure the UI is only on the client
    (bind _returnvalue (UserInterface|CreateWidget "/Game/_Main/UI/PlayerUI.PlayerUI_C"))
    (bind _output_get (Variables|Default|SetPlayerUI _returnvalue))
    (UserInterface|Viewport|AddtoViewport _output_get 0)))

(event EventUpdateHungerUI
  (params (NewHunger :type Float%20%28single-precision%29))
  (Default|UpdateHunger (Variables|Default|GetPlayerUI) NewHunger))

(event EventUpdateThirstUI
  (params (NewThirst :type Float%20%28single-precision%29))
  (Default|UpdateThirst (Variables|Default|GetPlayerUI) NewThirst))

(event EventInventoryMenu
  (params (Pickup :type Actor%20Class%20Reference) (Action :type E_ItemActions%20Enum :default "NewEnumerator0") (ItemWidget :type W%20Item%20Object%20Reference))
  (switch Utilities|FlowControl|Switch|SwitchonE_ItemActions Action
    (:NewEnumerator1
      (Default|InventoryRemoveItem(Server) (Variables|Default|GetAC_Inventory) (Variables|/Game/Inventory/UI/W_Item.W_Item_C|GetItem ItemWidget)))))

(event EventAddtoInventory
  (params (Pickup :type Actor%20Object%20Reference))
  (bind _itemid (Class|INTPickup|GetPickupInfo(Message) Pickup))
  (bind _outrownames (DataTable|GetDataTableRowNames "/Game/Inventory/DT_Items.DT_Items"))
  (bind _returnvalue (Utilities|GetDataTableRow "/Game/Inventory/DT_Items.DT_Items" (Utilities|Array|Get(acopy) _outrownames (- _itemid 1)))
    (:then
      (CallFunction|ServerAddInventoryItem _returnvalue Pickup))))

(event EventDropInventoryItem
  (params (ItemToDrop :type Actor%20Class%20Reference))
  (Game|SpawnActorfromClass ItemToDrop (Transformation|GetActorTransform (Pawn|GetControlledPawn)) "AlwaysSpawn" 0 0))

(event EventUpdateAmmoUI
  (params (NewAmmo :type Integer))
  (CallFunction|ClientUpdateAmmoUI NewAmmo))

(event EventSetMaxAmmoUI
  (params (MaxAmmo :type Integer))
  (CallFunction|ClientSetMaxAmmoUI MaxAmmo))

(event Input|ActionEvents|InputActionInventory
  (params (Key :type Key%20Structure :default "None"))
  (bind _ac_inventory (Variables|Default|GetAC_Inventory))
  (bind _inventorywidget (Variables|/Game/Inventory/AC_Inventory.AC_Inventory_C|GetInventoryWidget _ac_inventory))
  (:Pressed
    (if (not (Variables|Default|GetInventoryOpen))
      (UserInterface|Viewport|AddtoViewport _inventorywidget 0)
      (Variables|Default|SetInventoryOpen true)
      (Input|SetInputModeGameandUI self _inventorywidget "DoNotLock" true)
      (Variables|Default|SetbShowMouseCursor true)
      (else
        (Widget|RemovefromParent _inventorywidget)
        (Variables|Default|SetInventoryOpen false)
        (Input|SetInputModeGameOnly)
        (Variables|Default|SetbShowMouseCursor false)))))

(fn ConstructionScript)

(fn SurvivalControllerRef
  (return self))